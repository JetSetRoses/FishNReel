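; BP_KeyCard is a key card pickup that animates in place and vanishes when the player touches it.
; Tick spins it by a fixed yaw step per frame, while an endlessly looping yoyo vector tween started at BeginPlay moves it between its start location and an Offset.
; Overlap of its Sphere by the player pawn destroys the actor, with no key state recorded here.
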(event OnComponentBeginOverlap(Sphere)
  (params (OverlappedComponent :type Primitive%20Component%20Object%20Reference) (OtherActor :type Actor%20Object%20Reference) (OtherComp :type Primitive%20Component%20Object%20Reference) (OtherBodyIndex :type Integer) (bFromSweep :type Boolean) (SweepResult :type Hit%20Result%20Structure%20%28by%20ref%29))
  (if (== OtherActor (Game|Player|GetPlayerPawn 0))
    (Actor|DestroyActor)))

(event EventBeginPlay
  (bind _returnvalue (Transformation|GetActorLocation))
  (bind _value (|TweenVector _returnvalue (+ _returnvalue (Variables|Default|Getoffset)) 1.0 "InOutQuad" 0.0 0.0 0.0 -1 0.0 true)
    (:ApplyEasing
      (Transformation|SetActorLocation _value false false))))

(event Collision|EventActorBeginOverlap
  (params (OtherActor :type Actor%20Object%20Reference)))

(event EventTick
  (params (DeltaSeconds :type Float%20%28single-precision%29))
  (Transformation|AddActorLocalRotation "0.000000,0.500000,0.000000" false false))

(fn ConstructionScript)