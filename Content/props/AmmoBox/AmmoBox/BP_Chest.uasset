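; Interactable chest prop whose lid swings open when the player presses E while inside its overlap sphere.
; The sphere's overlap events track whether the player pawn is in range.
; Opening runs a yoyo rotation tween with a bounce ease, adding an offset rotation to the lid, then returning it after a short delay.
; A CanInteract flag blocks re-triggering until the tween completes.
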(event OnComponentBeginOverlap(Sphere)
  (params (OverlappedComponent :type Primitive%20Component%20Object%20Reference) (OtherActor :type Actor%20Object%20Reference) (OtherComp :type Primitive%20Component%20Object%20Reference) (OtherBodyIndex :type Integer) (bFromSweep :type Boolean) (SweepResult :type Hit%20Result%20Structure%20%28by%20ref%29))
  (if (== OtherActor (Game|Player|GetPlayerPawn 0))
    (Variables|Default|SetplayeInRange true)))

(event OnComponentEndOverlap(Sphere)
  (params (OverlappedComponent :type Primitive%20Component%20Object%20Reference) (OtherActor :type Actor%20Object%20Reference) (OtherComp :type Primitive%20Component%20Object%20Reference) (OtherBodyIndex :type Integer))
  (if (== OtherActor (Game|Player|GetPlayerPawn 0))
    (Variables|Default|SetplayeInRange false)))

(event Custom|OpenChest
  (bind _sm_chestlid (Variables|Default|GetSM_ChestLid))
  (bind _relativerotation (Variables|/Script/Engine.SceneComponent|GetRelativeRotation _sm_chestlid))
  (if (and (Variables|Default|GetplayeInRange) (Variables|Default|GetcanInteract))
    (bind _value (|TweenRotator _relativerotation (Math|Rotator|CombineRotators _relativerotation (Variables|Default|GetoffsetRotation)) (Variables|Default|GetopenTime) "OutBounce" 0.0 0.0 0.0 1 0.0 true 2.0)
      (:then
        (Variables|Default|SetcanInteract false))
      (:ApplyEasing
        (Transformation|SetRelativeRotation (Variables|Default|GetSM_ChestLid) _value false false))
      (:OnComplete
        (Variables|Default|SetcanInteract true)))))

(event EventBeginPlay
  (Variables|Default|SetcanInteract true))

(event Input|KeyboardEvents|E
  (params (Key :type Key%20Structure :default "None"))
  (:Pressed
    (CallFunction|OpenChest)))

(fn ConstructionScript)