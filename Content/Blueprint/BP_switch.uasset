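; BP_switch is an overlap-triggered switch that opens a linked door and shows a one-time camera cutscene.
; Each first-person character overlap with its Box calls OpenDoor on PuertaTarget.
; The player's first overlap also pauses the game and blends the view to CameraToFocus.
; A TweenFloat that ticks during pause acts as a timer, then blends back to the pawn and unpauses.
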(event OnComponentBeginOverlap(Box)
  (params (OverlappedComponent :type Primitive%20Component%20Object%20Reference) (OtherActor :type Actor%20Object%20Reference) (OtherComp :type Primitive%20Component%20Object%20Reference) (OtherBodyIndex :type Integer) (bFromSweep :type Boolean) (SweepResult :type Hit%20Result%20Structure%20%28by%20ref%29))
  (Utilities|Casting|CastToBP_FirstPersonCharacter OtherActor)
  (Default|OpenDoor (Variables|Default|GetPuertaTarget))
  (if (and (== OtherActor (Game|Player|GetPlayerPawn 0)) (not (Variables|Default|GetisPressed)))
    (CallFunction|Camerasequence)
    (Variables|Default|SetisPressed true)
    (Game|SetGamePaused true)))

(event Custom|camerasequence
  (Game|Player|SetViewTargetwithBlend (Game|GetPlayerController 0) (Variables|Default|GetcameraToFocus) 2.0 "VTBlend_Linear" 0.0 false)
  (|TweenFloat 0.0 1.0 5.0 "InOutQuad" 0.0 0.0 0.0 0 0.0 false 0.0 true
    (:OnComplete
      (CallFunction|Returntoplayercam)
      (Game|SetGamePaused false))))

(event Custom|returntoplayercam
  (bind _returnvalue (Game|GetPlayerController 0))
  (Game|Player|SetViewTargetwithBlend _returnvalue (Pawn|GetControlledPawn _returnvalue) 2.0 "VTBlend_Linear" 0.0 false))

(event EventBeginPlay)

(event Collision|EventActorBeginOverlap
  (params (OtherActor :type Actor%20Object%20Reference)))

(event EventTick
  (params (DeltaSeconds :type Float%20%28single-precision%29)))

(fn ConstructionScript)