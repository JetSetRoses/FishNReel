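; MeleeBP is a melee weapon Blueprint that plays a Paper2D attack animation when its Shoot event fires.
; Shoot calls Fireweapon, switches the flipbook to the full melee animation, waits for its length, then returns to the idle flipbook.
; A DoOnce gate resets only after that delay, so repeated Shoot calls are ignored until the swing finishes.
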(event EventBeginPlay
  (|CallParentFunction) ; This node is disabled and will not be called.\nDrag off pins to build functionality.
)

(event Collision|EventActorBeginOverlap
  (params (OtherActor :type Actor%20Object%20Reference))
  (|CallParentFunction OtherActor) ; This node is disabled and will not be called.\nDrag off pins to build functionality.
)

(event EventTick
  (params (DeltaSeconds :type Float%20%28single-precision%29))
  (|CallParentFunction DeltaSeconds) ; This node is disabled and will not be called.\nDrag off pins to build functionality.
)

(event EventShoot
  (bind _paperflipbook (Variables|Default|GetPaperFlipbook))
  (Utilities|FlowControl|DoOnce false
    (:Completed
      (CallFunction|Fireweapon)
      (Sprite|SetFlipbook _paperflipbook "/Game/fps/RetroFPSAssets/Weapons/Chainsaw/melee_full.melee_full")
      (Utilities|FlowControl|Delay (Class|PaperFlipbookComponent|GetFlipbookLength _paperflipbook))
      (Sprite|SetFlipbook (Variables|Default|GetPaperFlipbook) "/Game/fps/RetroFPSAssets/Weapons/Chainsaw/melee_idle.melee_idle")
      (Class|TypedElementListLibrary|Reset))))

(fn ConstructionScript
  (|CallParentFunction))