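; Base weapon actor for a first-person shooter, with empty shoot and stopshooting events and shared firing and ammo logic.
; Fireweapon plays a camera shake, line-traces forward from the Line component and applies Weapondamage to the hit actor.
; Ammo lives on the player character cached at BeginPlay; HasAmmo checks and DecreaseAmmo decrements the Bullet or Shell count by AmmoType, updating the player's UI.
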(event Custom|DecreaseAmmo
  (bind _player_ref (Variables|Default|Getplayer%20Ref))
  (bind _player_ref_2 (Variables|Default|Getplayer%20Ref))
  (switch Utilities|FlowControl|Switch|SwitchonAmmoEnum (Variables|Default|GetAmmoType)
    (:NewEnumerator0
      (Math|Integer|DecrementInt (Variables|/Game/FirstPerson/Blueprints/BP_FirstPersonCharacter.BP_FirstPersonCharacter_C|Getbullet _player_ref)
        (:%20%20
          (Default|UpdateBullet (Variables|/Game/FirstPerson/Blueprints/BP_FirstPersonCharacter.BP_FirstPersonCharacter_C|GetUI_Ref _player_ref)))))
    (:NewEnumerator1
      (Math|Integer|DecrementInt (Variables|/Game/FirstPerson/Blueprints/BP_FirstPersonCharacter.BP_FirstPersonCharacter_C|GetShell _player_ref_2)
        (:%20%20
          (Default|UpdateShells (Variables|/Game/FirstPerson/Blueprints/BP_FirstPersonCharacter.BP_FirstPersonCharacter_C|GetUI_Ref _player_ref_2)))))))

(event Custom|shoot)

(event Custom|stop%20shooting)

(event EventBeginPlay
  (bind _asbp_first_person_character (Utilities|Casting|CastToBP_FirstPersonCharacter (Game|GetPlayerCharacter 0)))
  (Variables|Default|Setplayer%20Ref _asbp_first_person_character))

(event Collision|EventActorBeginOverlap
  (params (OtherActor :type Actor%20Object%20Reference)))

(event EventTick
  (params (DeltaSeconds :type Float%20%28single-precision%29)))

(fn ConstructionScript)

(fn Fireweapon
  (bind _line (Variables|Default|Getline))
  (bind _returnvalue (Transformation|GetWorldLocation _line))
  (CameraShakes|StartCameraShake (Variables|/Script/Engine.PlayerController|GetPlayerCameraManager (Game|GetPlayerController 0)) (Variables|Default|GetWeapon%20Shake) 0.5 "CameraLocal" "0, 0, 0")
  (bind (_outhit _returnvalue_2) (Collision|LineTraceForObjects _returnvalue (+ _returnvalue (* (Math|Vector|GetForwardVector (Transformation|GetWorldRotation _line)) (Variables|Default|Getfiredistance))) (Utilities|Array|MakeArray "ObjectTypeQuery1" "ObjectTypeQuery2" "ObjectTypeQuery3") false (Utilities|Array|MakeArray self (Game|GetPlayerCharacter 0)) "None"))
  (if _returnvalue_2
    (Game|Damage|ApplyDamage (.HitActor (Collision|BreakHitResult _outhit)) (Variables|Default|Getweapondamage) 0 0)))

(fn HasAmmo?
  (switch Utilities|FlowControl|Switch|SwitchonAmmoEnum (Variables|Default|GetAmmoType)
    (:NewEnumerator0
      (if (> (Variables|/Game/FirstPerson/Blueprints/BP_FirstPersonCharacter.BP_FirstPersonCharacter_C|Getbullet (Variables|Default|Getplayer%20Ref)) 0)
        (return true)
        (else
          (return false))))
    (:NewEnumerator1
      (if (> (Variables|/Game/FirstPerson/Blueprints/BP_FirstPersonCharacter.BP_FirstPersonCharacter_C|GetShell (Variables|Default|Getplayer%20Ref)) 0)
        (return true)
        (else
          (return false))))))