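; Pistol weapon Blueprint with flipbook animation, ammo-checked firing and material effects.
; Shoot uses a DoOnce gate to fire, decrease ammo, play sound and camera shake, then resets after the shoot flipbook finishes.
; BeginPlay creates a dynamic sprite material, whose TintMask and Dither parameters are tweened for flicker and fade effects on the Q and B keys.
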(event Custom|reset
  (bind _paperflipbook (Variables|Default|GetPaperFlipbook))
  (Utilities|FlowControl|DoOnce false) ; enters at Reset
)

(event Custom|CreateRuntimeMaterial
  (bind _returnvalue (Rendering|Material|CreateDynamicMaterialInstance (Variables|Default|GetPaperFlipbook) 0 "/Game/material/MM_SpriteMaterial.MM_SpriteMaterial" "None" :!class /Script/Engine.PrimitiveComponent))
  (Variables|Default|SetRuntimeMat _returnvalue))

(event Custom|flickr
  (Rendering|Material|SetScalarParameterValue (Variables|Default|GetRuntimeMat) (Variables|Default|GetTintMask) 0.0 :!class /Script/Engine.MaterialInstanceDynamic)
  (bind _returnvalue (Rendering|Material|GetScalarParameterValue (Variables|Default|GetRuntimeMat) (Variables|Default|GetTintMask) :!class /Script/Engine.MaterialInstanceDynamic))
  (bind _value (|TweenFloat _returnvalue 1.0 0.2 "InOutQuad" 0.0 0.0 0.0 4 0.0 true)
    (:ApplyEasing
      (Rendering|Material|SetScalarParameterValue (Variables|Default|GetRuntimeMat) (Variables|Default|GetTintMask) _value :!class /Script/Engine.MaterialInstanceDynamic))))

(event Custom|fade
  (bind _returnvalue (Rendering|Material|GetScalarParameterValue (Variables|Default|GetRuntimeMat) (Variables|Default|GetDither) :!class /Script/Engine.MaterialInstanceDynamic))
  ;[0.15 0.15 0.15 0.5] para el enemigo le pones destroy despues de on complete
  (bind _value (|TweenFloat _returnvalue 0.0 0.5 "InOutQuad")
    (:ApplyEasing
      (Rendering|Material|SetScalarParameterValue (Variables|Default|GetRuntimeMat) (Variables|Default|GetDither) _value :!class /Script/Engine.MaterialInstanceDynamic))))

(event EventBeginPlay
  (|CallParentFunction)
  (CallFunction|CreateRuntimeMaterial))

(event Collision|EventActorBeginOverlap
  (params (OtherActor :type Actor%20Object%20Reference))
  (|CallParentFunction OtherActor) ; This node is disabled and will not be called.\nDrag off pins to build functionality.
)

(event EventTick
  (params (DeltaSeconds :type Float%20%28single-precision%29))
  (|CallParentFunction DeltaSeconds) ; This node is disabled and will not be called.\nDrag off pins to build functionality.
)

(event EventShoot
  (bind _paperflipbook (Variables|Default|GetPaperFlipbook))
  (bind _hasammo (CallFunction|HasAmmo?))
  (if _hasammo
    (Utilities|FlowControl|DoOnce false
      (:Completed
        (CallFunction|DecreaseAmmo)
        (CallFunction|Fireweapon)
        (Audio|PlaySoundatLocation "/Game/ShooterSFX/SC_GunShot.SC_GunShot" (Transformation|GetActorLocation) "0, 0, 0" 1.0 1.0 0.0 0 0 0 0)
        (CameraShakes|StartCameraShake (Variables|/Script/Engine.PlayerController|GetPlayerCameraManager (Game|GetPlayerController 0)) "/Game/Blueprint/camerashake/BP_Gunshake.BP_Gunshake_C" 1.0 "CameraLocal" "0, 0, 0")
        (Sprite|SetFlipbook _paperflipbook "/Game/fps/RetroFPSAssets/Weapons/Pistol/gun_shoot.gun_shoot")
        (Utilities|FlowControl|Delay (Class|PaperFlipbookComponent|GetFlipbookLength _paperflipbook))
        (Sprite|SetFlipbook (Variables|Default|GetPaperFlipbook) "/Game/fps/RetroFPSAssets/Weapons/Pistol/gun_idle.gun_idle")
        (CallFunction|Reset)))))

(event Input|KeyboardEvents|Q
  (params (Key :type Key%20Structure :default "None"))
  (:Pressed
    (CallFunction|Flickr)))

(event Input|KeyboardEvents|B
  (params (Key :type Key%20Structure :default "None"))
  (:Pressed
    (CallFunction|Fade)))

(fn ConstructionScript
  (|CallParentFunction))