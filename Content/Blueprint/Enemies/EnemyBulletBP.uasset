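; EnemyBulletBP is an enemy projectile that hurts the player on contact.
; When its sphere overlaps a Player-tagged actor, it calls ApplyDamage on player controller 0 and plays a hurt sound.
; For a BP_FirstPersonCharacter, a DoOnce-gated step also directly lowers clamped Health, refreshes the player UI, stops projectile movement and destroys the bullet.
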(event OnComponentBeginOverlap(Sphere1)
  (params (OverlappedComponent :type Primitive%20Component%20Object%20Reference) (OtherActor :type Actor%20Object%20Reference) (OtherComp :type Primitive%20Component%20Object%20Reference) (OtherBodyIndex :type Integer) (bFromSweep :type Boolean) (SweepResult :type Hit%20Result%20Structure%20%28by%20ref%29))
  (if (Actor|ActorHasTag OtherActor "Player")
    (Game|Damage|ApplyDamage (Game|GetPlayerController 0) 1e+01 0 0)
    (Audio|PlaySoundatLocation "/Game/ShooterSFX/SC_Hurt.SC_Hurt" (Transformation|GetActorLocation) "0, 0, 0" 1.0 1.0 0.0 0 0 0 0)
    (bind _asbp_first_person_character (Utilities|Casting|CastToBP_FirstPersonCharacter OtherActor))
    (Utilities|FlowControl|DoOnce false
      (:Completed
        (Variables|/Game/FirstPerson/Blueprints/BP_FirstPersonCharacter.BP_FirstPersonCharacter_C|SetHealth _asbp_first_person_character (Math|Float|Clamp(Float) (- (Variables|/Game/FirstPerson/Blueprints/BP_FirstPersonCharacter.BP_FirstPersonCharacter_C|GetHealth _asbp_first_person_character) 5.0) 0.0 (Variables|/Game/FirstPerson/Blueprints/BP_FirstPersonCharacter.BP_FirstPersonCharacter_C|GetmaxHealth _asbp_first_person_character)))
        (Default|UpdatePlayerInfo (Variables|/Game/FirstPerson/Blueprints/BP_FirstPersonCharacter.BP_FirstPersonCharacter_C|GetUI_Ref _asbp_first_person_character))
        (Components|Movement|StopMovementImmediately (Variables|Default|GetProjectileMovement))
        (Actor|DestroyActor)))))

(event EventBeginPlay)

(event Collision|EventActorBeginOverlap
  (params (OtherActor :type Actor%20Object%20Reference)))

(event EventTick
  (params (DeltaSeconds :type Float%20%28single-precision%29)))

(fn ConstructionScript)