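; Enemy pawn drawn as a directional Paper2D flipbook sprite, with projectile and line-trace melee attacks.
; PawnSensing sets a timed CanSeePlayer blackboard flag and makes it turn toward the player.
; Tick derives its state from velocity and attack flags, then picks one of eight flipbooks by dot-product angle to the player.
; Damage flickers the material tint; death stops AI, plays death flipbooks and notifies the game mode, while the dither fade is unconnected.
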(event OnSeePawn(PawnSensing)
  (params (Pawn :type Pawn%20Object%20Reference))
  (Utilities|Casting|CastToBP_FirstPersonCharacter Pawn)
  (Variables|Default|SetCanSeePlayer true)
  (AI|Components|Blackboard|SetValueasBool (AI|GetBlackboard 0) (Utilities|Name|MakeLiteralName "CanSeePlayer") true)
  (Utilities|FlowControl|RetriggerableDelay 0.7)
  (Variables|Default|SetCanSeePlayer false)
  (AI|Components|Blackboard|SetValueasBool (AI|GetBlackboard 0) (Utilities|Name|MakeLiteralName "CanSeePlayer") false))

(event Custom|rotateTowardsPlayer
  (Transformation|SetActorRotation (Math|Interpolation|RInterpTo (Transformation|GetActorRotation) (Math|Rotator|FindLookatRotation (Transformation|GetActorLocation) (Transformation|GetActorLocation (Game|GetPlayerCharacter 0))) (Utilities|Time|GetWorldDeltaSeconds) 1e+01)))

(event Custom|SpawnProjectile
  (Variables|Default|SetisAttacking true)
  (Variables|Default|SetAttackState "NewEnumerator1")
  (Components|Movement|StopMovementImmediately (Variables|Character|GetCharacterMovement))
  (Utilities|FlowControl|RetriggerableDelay 0.5)
  (Game|SpawnActorfromClass "/Game/Blueprint/Enemies/EnemyBulletBP.EnemyBulletBP_C" (Transformation|GetWorldTransform (Variables|Default|GetSpawnPoint)) "Undefined" "MultiplyWithRoot" 0 0))

(event Custom|flickr
  (Rendering|Material|SetScalarParameterValue (Variables|Default|GetRuntime%20Mat) (Variables|Default|GetTint%20mask) 0.0 :!class /Script/Engine.MaterialInstanceDynamic)
  (bind _returnvalue (Rendering|Material|GetScalarParameterValue (Variables|Default|GetRuntime%20Mat) (Variables|Default|GetTint%20mask) :!class /Script/Engine.MaterialInstanceDynamic))
  (bind _value (|TweenFloat _returnvalue 1.0 0.2 "InOutQuad" 0.0 0.0 0.0 4 0.0 true)
    (:ApplyEasing
      (Rendering|Material|SetScalarParameterValue (Variables|Default|GetRuntime%20Mat) (Variables|Default|GetTint%20mask) _value :!class /Script/Engine.MaterialInstanceDynamic))))

(event Custom|fade
  (bind _returnvalue (Rendering|Material|GetScalarParameterValue (Variables|Default|GetRuntime%20Mat) (Variables|Default|GetDither) :!class /Script/Engine.MaterialInstanceDynamic))
  (bind _value (|TweenFloat _returnvalue 0.0 0.5 "InOutQuad")
    (:ApplyEasing
      (Rendering|Material|SetScalarParameterValue (Variables|Default|GetRuntime%20Mat) (Variables|Default|GetDither) _value :!class /Script/Engine.MaterialInstanceDynamic))
    (:OnComplete
      (Actor|DestroyActor))))

(event Custom|CreateRuntimeMaterial
  (bind _returnvalue (Rendering|Material|CreateDynamicMaterialInstance (Variables|Default|GetPaperFlipbook) 0 "/Game/material/MM_SpriteMaterial.MM_SpriteMaterial" "None" :!class /Script/Engine.PrimitiveComponent))
  (Variables|Default|SetRuntime%20Mat _returnvalue))

(event Custom|meleeattack
  (bind _returnvalue (Transformation|GetActorLocation))
  (Variables|Default|SetisAttacking true)
  (Variables|Default|SetAttackState "NewEnumerator0")
  (Utilities|FlowControl|RetriggerableDelay 0.5)
  (bind _outhit (Collision|LineTraceForObjects _returnvalue (+ _returnvalue (* (Transformation|GetActorForwardVector) 2e+02)) (Utilities|Array|MakeArray "ObjectTypeQuery3") false (Utilities|Array|MakeArray self) "None"))
  (if (== (.HitActor (Collision|BreakHitResult _outhit)) (Game|GetPlayerCharacter 0))
    (Game|Damage|ApplyDamage (.HitActor (Collision|BreakHitResult _outhit)) 5.0 0 0)))

(event Custom|handleDead
  (bind _paperflipbook (Variables|Default|GetPaperFlipbook))
  (Transformation|SetActorRotation (Math|Rotator|MakeRotator 0.0 0.0 (.yaw (Math|Rotator|FindLookatRotation (Transformation|GetActorLocation) (Transformation|GetActorLocation (Game|GetPlayerController 0))))))
  (Utilities|FlowControl|DoOnce false
    (:Completed
      (AI|Logic|StopLogic (Variables|/Script/AIModule.AIController|GetBrainComponent (AI|GetAIController self)) "")
      (Pawn|Components|CharacterMovement|SetMovementMode (Variables|Character|GetCharacterMovement) "MOVE_Flying" 0)
      (Collision|SetCollisionEnabled (Variables|Collision|GetCapsuleComponent) "NoCollision")
      (Components|Activation|Deactivate (Variables|Character|GetCharacterMovement))
      (Transformation|SetRelativeRotation _paperflipbook "0.000000,-90.000000,0.000000" false false)
      (Sprite|SetFlipbook _paperflipbook "/Game/Blueprint/Enemies/Sprites/Pez/Death/pez_muerte1.pez_muerte1")
      (Utilities|FlowControl|Delay (- (Class|PaperFlipbookComponent|GetFlipbookLength _paperflipbook) 0.0))
      (Transformation|AddActorLocalOffset "0.000000,0.000000,-30.000000" false false)
      (Sprite|SetFlipbook _paperflipbook "/Game/Blueprint/Enemies/Sprites/Pez/Death/pez_muerte_idle.pez_muerte_idle")
      (bind _asbp_first_person_game_mode (Utilities|Casting|CastToBP_FirstPersonGameMode (Game|GetGameMode)))
      (Default|RegisterEnemyDeath _asbp_first_person_game_mode))))

(event EventBeginPlay
  (CallFunction|CreateRuntimeMaterial))

(event EventTick
  (params (DeltaSeconds :type Float%20%28single-precision%29))
  (bind _returnvalue (Game|GetPlayerCharacter 0))
  (bind _returnvalue_2 (Transformation|GetActorLocation))
  (bind _isattacking (Variables|Default|GetisAttacking))
  (bind _returnvalue_3 (Transformation|GetActorLocation _returnvalue))
  (bind _returnvalue_4 (- _returnvalue_3 _returnvalue_2))
  (bind _returnvalue_5 (Math|Vector|Normalize _returnvalue_4))
  (if (> (Math|Vector|VectorLength (Variables|/Script/Engine.MovementComponent|GetVelocity (Variables|Character|GetCharacterMovement))) 0.0)
    (if _isattacking
      (switch Utilities|FlowControl|Switch|SwitchonEnemyAttack (Variables|Default|GetAttackState)
        (:NewEnumerator0
          (Variables|Default|SetEnemyState "NewEnumerator2"))
        (:NewEnumerator1
          (Variables|Default|SetEnemyState "NewEnumerator3")))
      (else
        (Variables|Default|SetEnemyState "NewEnumerator1")))
    (elif _isattacking
      (switch Utilities|FlowControl|Switch|SwitchonEnemyAttack (Variables|Default|GetAttackState)
        (:NewEnumerator0
          (Variables|Default|SetEnemyState "NewEnumerator2"))
        (:NewEnumerator1
          (Variables|Default|SetEnemyState "NewEnumerator3")))
      (else
        (Variables|Default|SetEnemyState "NewEnumerator0"))))
  (if (Variables|Default|GetIsDead)
    (CallFunction|HandleDead)
    (else
      (if (Variables|Default|GetCanSeePlayer)
        (CallFunction|RotateTowardsPlayer))
      (Variables|Default|Setdegrees (Class|KismetMathLibrary|DegAcos (Math|Vector|DotProduct (Transformation|GetActorForwardVector) _returnvalue_5)))
      (if (< (Math|Vector|DotProduct (Transformation|GetActorRightVector) _returnvalue_5) 0.0)
        (Math|Float|CompareFloat (Variables|Default|Getdegrees) 1.8e+02
          (:>
            (Transformation|SetRelativeRotation (Variables|Default|GetPaperFlipbook) "0.000000,-90.000000,0.000000" false false :!label _label)
            (Sprite|SetFlipbook (Variables|Default|GetPaperFlipbook) (Utilities|Array|Get(acopy) (Utilities|Select :Index (Variables|Default|GetEnemyState) :NewEnumerator0 (Variables|Default|GetidleFlipbook) :NewEnumerator1 (Variables|Default|GetmoveFlipbook) :NewEnumerator2 (Variables|Default|GetmeleeFlipbook) :NewEnumerator3 (Variables|Default|GetfireFlipbook)))))
          (:==
            (goto _label))
          (:<
            (Math|Float|CompareFloat (Variables|Default|Getdegrees) 135.0
              (:>
                (Transformation|SetRelativeRotation (Variables|Default|GetPaperFlipbook) "0.000000,135.000000,0.000000" false false :!label _label_2)
                (Sprite|SetFlipbook (Variables|Default|GetPaperFlipbook) (Utilities|Array|Get(acopy) (Utilities|Select :Index (Variables|Default|GetEnemyState) :NewEnumerator0 (Variables|Default|GetidleFlipbook) :NewEnumerator1 (Variables|Default|GetmoveFlipbook) :NewEnumerator2 (Variables|Default|GetmeleeFlipbook) :NewEnumerator3 (Variables|Default|GetfireFlipbook)) 1)))
              (:==
                (goto _label_2))
              (:<
                (Math|Float|CompareFloat (Variables|Default|Getdegrees) 9e+01
                  (:>
                    (Transformation|SetRelativeRotation (Variables|Default|GetPaperFlipbook) "0.000000,180.000000,0.000000" false false :!label _label_3)
                    (Sprite|SetFlipbook (Variables|Default|GetPaperFlipbook) (Utilities|Array|Get(acopy) (Utilities|Select :Index (Variables|Default|GetEnemyState) :NewEnumerator0 (Variables|Default|GetidleFlipbook) :NewEnumerator1 (Variables|Default|GetmoveFlipbook) :NewEnumerator2 (Variables|Default|GetmeleeFlipbook) :NewEnumerator3 (Variables|Default|GetfireFlipbook)) 2)))
                  (:==
                    (goto _label_3))
                  (:<
                    (Math|Float|CompareFloat (Variables|Default|Getdegrees) 45.0
                      (:>
                        _)
                      (:==
                        _)
                      (:<
                        (goto _label)))
                    (Transformation|SetRelativeRotation (Variables|Default|GetPaperFlipbook) "0.000000,45.000000,0.000000" false false)
                    (Sprite|SetFlipbook (Variables|Default|GetPaperFlipbook) (Utilities|Array|Get(acopy) (Utilities|Select :Index (Variables|Default|GetEnemyState) :NewEnumerator0 (Variables|Default|GetidleFlipbook) :NewEnumerator1 (Variables|Default|GetmoveFlipbook) :NewEnumerator2 (Variables|Default|GetmeleeFlipbook) :NewEnumerator3 (Variables|Default|GetfireFlipbook)) 3))))))))
        (else
          (Math|Float|CompareFloat (Variables|Default|Getdegrees) 1.8e+02
            (:>
              (Transformation|SetRelativeRotation (Variables|Default|GetPaperFlipbook) "0.000000,-45.000000,0.000000" false false :!label _label_4)
              (Sprite|SetFlipbook (Variables|Default|GetPaperFlipbook) (Utilities|Array|Get(acopy) (Utilities|Select :Index (Variables|Default|GetEnemyState) :NewEnumerator0 (Variables|Default|GetidleFlipbook) :NewEnumerator1 (Variables|Default|GetmoveFlipbook) :NewEnumerator2 (Variables|Default|GetmeleeFlipbook) :NewEnumerator3 (Variables|Default|GetfireFlipbook)) 4)))
            (:==
              (goto _label_4))
            (:<
              (Math|Float|CompareFloat (Variables|Default|Getdegrees) 135.0
                (:>
                  (Transformation|SetRelativeRotation (Variables|Default|GetPaperFlipbook) "0.000000,90.000000,0.000000" false false :!label _label_5)
                  (Sprite|SetFlipbook (Variables|Default|GetPaperFlipbook) (Utilities|Array|Get(acopy) (Utilities|Select :Index (Variables|Default|GetEnemyState) :NewEnumerator0 (Variables|Default|GetidleFlipbook) :NewEnumerator1 (Variables|Default|GetmoveFlipbook) :NewEnumerator2 (Variables|Default|GetmeleeFlipbook) :NewEnumerator3 (Variables|Default|GetfireFlipbook)) 5)))
                (:==
                  (goto _label_5))
                (:<
                  (Math|Float|CompareFloat (Variables|Default|Getdegrees) 9e+01
                    (:>
                      (Transformation|SetRelativeRotation (Variables|Default|GetPaperFlipbook) "0.000000,45.000000,0.000000" false false :!label _label_6)
                      (Sprite|SetFlipbook (Variables|Default|GetPaperFlipbook) (Utilities|Array|Get(acopy) (Utilities|Select :Index (Variables|Default|GetEnemyState) :NewEnumerator0 (Variables|Default|GetidleFlipbook) :NewEnumerator1 (Variables|Default|GetmoveFlipbook) :NewEnumerator2 (Variables|Default|GetmeleeFlipbook) :NewEnumerator3 (Variables|Default|GetfireFlipbook)) 6)))
                    (:==
                      (goto _label_6))
                    (:<
                      (Math|Float|CompareFloat (Variables|Default|Getdegrees) 45.0
                        (:>
                          _)
                        (:==
                          _)
                        (:<
                          (goto _label_4)))
                      (Transformation|SetRelativeRotation (Variables|Default|GetPaperFlipbook) "0, 0, 0" false false)
                      (Sprite|SetFlipbook (Variables|Default|GetPaperFlipbook) (Utilities|Array|Get(acopy) (Utilities|Select :Index (Variables|Default|GetEnemyState) :NewEnumerator0 (Variables|Default|GetidleFlipbook) :NewEnumerator1 (Variables|Default|GetmoveFlipbook) :NewEnumerator2 (Variables|Default|GetmeleeFlipbook) :NewEnumerator3 (Variables|Default|GetfireFlipbook)) 7)))))))))))))

(event Game|Damage|EventAnyDamage
  (params (Damage :type Float%20%28single-precision%29) (DamageType :type Damage%20Type%20Object%20Reference) (InstigatedBy :type Controller%20Object%20Reference) (DamageCauser :type Actor%20Object%20Reference))
  (bind _output_get (Variables|Default|SetHealth (- (Variables|Default|GetHealth) Damage)))
  (if (<= _output_get 0.0)
    (Variables|Default|SetIsDead true)
    (else
      (CallFunction|Flickr))))

(fn ConstructionScript)