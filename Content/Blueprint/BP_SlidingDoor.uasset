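; BP_SlidingDoor is a door the player slides open by pressing G while inside its sphere trigger.
; The sphere overlap tracks the player pawn and enables or disables the actor's input.
; A TweenVector with sine easing moves the door mesh by OffsetLocation over OpenTime, blocking re-triggering until it completes.
; Each activation offsets from the current relative location, with no closing logic.
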(event OnComponentBeginOverlap(Sphere)
  (params (OverlappedComponent :type Primitive%20Component%20Object%20Reference) (OtherActor :type Actor%20Object%20Reference) (OtherComp :type Primitive%20Component%20Object%20Reference) (OtherBodyIndex :type Integer) (bFromSweep :type Boolean) (SweepResult :type Hit%20Result%20Structure%20%28by%20ref%29))
  (if (== OtherActor (Game|Player|GetPlayerPawn 0))
    (Variables|Default|SetplayerInRange true)
    (Input|EnableInput (Game|GetPlayerController 0))))

(event OnComponentEndOverlap(Sphere)
  (params (OverlappedComponent :type Primitive%20Component%20Object%20Reference) (OtherActor :type Actor%20Object%20Reference) (OtherComp :type Primitive%20Component%20Object%20Reference) (OtherBodyIndex :type Integer))
  (if (== OtherActor (Game|Player|GetPlayerPawn 0))
    (Variables|Default|SetplayerInRange false)
    (Input|DisableInput (Game|GetPlayerController 0))))

(event Custom|openDoor
  (bind _sm_door (Variables|Default|GetSM_Door))
  (bind _relativelocation (Variables|/Script/Engine.SceneComponent|GetRelativeLocation _sm_door))
  (if (and (Variables|Default|GetcanInteract) (Variables|Default|GetplayerInRange))
    (bind _value (|TweenVector _relativelocation (+ _relativelocation (Variables|Default|GetoffsetLocation)) (Variables|Default|GetopenTime) "InOutSine" 0.0 0.0 0.0 1)
      (:then
        (Variables|Default|SetcanInteract false))
      (:ApplyEasing
        (Transformation|SetRelativeLocation (Variables|Default|GetSM_Door) _value false false))
      (:OnComplete
        (Variables|Default|SetcanInteract true)))))

(event EventBeginPlay
  (Variables|Default|SetcanInteract true))

(event Input|KeyboardEvents|G
  (params (Key :type Key%20Structure :default "None"))
  (:Pressed
    (CallFunction|OpenDoor)))

(fn ConstructionScript)