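; Chest Blueprint whose lid swings open when OpenChest is called with the player in range.
; A yoyo rotator tween eases the lid by OffsetRotation over OpenTime, with CanInteract blocking retriggers until completion.
; A sphere's begin overlap sets PlayerInRange for the player pawn.
; End overlap is unwired, so PlayerInRange stays true once set.
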(event OnComponentBeginOverlap(Sphere)
  (params (OverlappedComponent :type Primitive%20Component%20Object%20Reference) (OtherActor :type Actor%20Object%20Reference) (OtherComp :type Primitive%20Component%20Object%20Reference) (OtherBodyIndex :type Integer) (bFromSweep :type Boolean) (SweepResult :type Hit%20Result%20Structure%20%28by%20ref%29))
  ;[0.15 0.15 0.15 0.5] Detectar si el jugador está cerca o no xdd
  (if (== OtherActor (Game|Player|GetPlayerPawn 0))
    (Variables|Default|SetplayerInRange true)))

(event OnComponentEndOverlap(Sphere)
  (params (OverlappedComponent :type Primitive%20Component%20Object%20Reference) (OtherActor :type Actor%20Object%20Reference) (OtherComp :type Primitive%20Component%20Object%20Reference) (OtherBodyIndex :type Integer))
  ;[0.15 0.15 0.15 0.5] Detectar si el jugador está cerca o no xdd
)

(event Custom|OpenChest
  (bind _sm_chestlid (Variables|Default|GetSM_ChestLid))
  (bind _relativerotation (Variables|/Script/Engine.SceneComponent|GetRelativeRotation _sm_chestlid))
  (if (and (Variables|Default|GetplayerInRange) (Variables|Default|GetCanInteract))
    (bind _value (|TweenRotator _relativerotation (Math|Rotator|CombineRotators _relativerotation (Variables|Default|GetoffsetRotation)) (Variables|Default|GetopenTime) "InOutQuad" 0.0 0.0 0.0 1 0.0 true)
      (:then
        (Variables|Default|SetCanInteract false))
      (:ApplyEasing
        (Transformation|SetRelativeRotation (Variables|Default|GetSM_ChestLid) _value false false))
      (:OnComplete
        (Variables|Default|SetCanInteract true)))))

(event EventBeginPlay
  ;[0.15 0.15 0.15 0.5] Al inicio es interactuable
  (Variables|Default|SetCanInteract true))

(fn ConstructionScript)