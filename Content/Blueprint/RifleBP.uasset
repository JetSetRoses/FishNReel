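; Rifle weapon Blueprint with a Paper2D flipbook sprite that handles firing and its animation.
; Shoot checks for ammo, then passes through a DoOnce gate to decrease ammo and call Fireweapon, neither of which is defined here.
; It plays the firing flipbook, waits for its length, returns to idle and calls Reset to reopen the gate, so the animation length limits fire rate.
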(event Custom|reset
  (bind _paperflipbook (Variables|Default|GetPaperFlipbook))
  (Utilities|FlowControl|DoOnce false) ; enters at Reset
)

(event EventBeginPlay
  (|CallParentFunction) ; This node is disabled and will not be called.\nDrag off pins to build functionality.
)

(event Collision|EventActorBeginOverlap
  (params (OtherActor :type Actor%20Object%20Reference))
  (|CallParentFunction OtherActor) ; This node is disabled and will not be called.\nDrag off pins to build functionality.
)

(event EventTick
  (params (DeltaSeconds :type Float%20%28single-precision%29))
  (|CallParentFunction DeltaSeconds) ; This node is disabled and will not be called.\nDrag off pins to build functionality.
)

(event EventShoot
  (bind _paperflipbook (Variables|Default|GetPaperFlipbook))
  (bind _hasammo (CallFunction|HasAmmo?))
  (if _hasammo
    (Utilities|FlowControl|DoOnce false
      (:Completed
        (CallFunction|DecreaseAmmo)
        (CallFunction|Fireweapon)
        (Sprite|SetFlipbook _paperflipbook "/Game/fps/RetroFPSAssets/Weapons/PlasmaGun/rifle_full.rifle_full")
        (Utilities|FlowControl|Delay (Class|PaperFlipbookComponent|GetFlipbookLength _paperflipbook))
        (Sprite|SetFlipbook (Variables|Default|GetPaperFlipbook) "/Game/fps/RetroFPSAssets/Weapons/PlasmaGun/rifle_idle.rifle_idle")
        (CallFunction|Reset)))))

(fn ConstructionScript
  (|CallParentFunction))